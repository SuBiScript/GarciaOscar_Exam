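; Trigger actor that plays a level sequence when the ThirdPersonCharacter overlaps it.
; BeginPlay creates and stores the sequence player; each qualifying overlap disables player input and plays it, with no replay check or input restore here.
; It stores a message, creates a TextToDisplay_BP widget referencing itself and fires that widget's feedback notification.
; A FlipFlop alternates between two sounds, each given a random pitch.
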(event `self.ReceiveBeginPlay`
  ;[1 1 1] Create Level sequencer and store it
  (bind (_outactor _returnvalue) (`LevelSequencePlayer.CreateLevelSequencePlayer` "/Game/Blueprints/Sequence/LevelSequence.LevelSequence"))
  (set `self.Sequence` _returnvalue))

(event `self.ReceiveActorBeginOverlap`
  (params (OtherActor :type "Actor Object Reference"))
  (bind _returnvalue (`KismetMathLibrary.RandomFloatInRange` 0.5 1.0))
  ;[1 1 1] Check if Sequence can be played or has already been
  (cast `/Game/ThirdPersonBP/Blueprints/ThirdPersonCharacter` OtherActor)
  (`self.DisableInput` (`GameplayStatics.GetPlayerCharacter` 0) null)
  (`MovieSceneSequencePlayer.Play` (`self.Sequence`))
  (`self.Display Message Sequence` "PLAYING SEQUENCE!")
  (bind _foundwidgets (`WidgetBlueprintLibrary.GetAllWidgetsOfClass` "/Game/Blueprints/HUD/TextToDisplay_BP.TextToDisplay_BP_C"))
  (`/Game/Blueprints/HUD/TextToDisplay_BP.FeedbackDisplayNotification` _foundwidgets)
  (`/Engine/EditorBlueprintResources/StandardMacros.FlipFlop`
    (:`A`
      (`AudioComponent.Play` (`self.Sequence_0`) 0.0)
      (`AudioComponent.SetPitchMultiplier` (`self.Sequence_0`) _returnvalue))
    (:`B`
      (`AudioComponent.Play` (`self.Sequence_1`) 0.0)
      (`AudioComponent.SetPitchMultiplier` (`self.Sequence_1`) _returnvalue))))

(fn `Display Message Sequence`
  (params (Message :type Text))
  (set `self.DisplayMessage` Message)
  (bind _returnvalue (`|CreateWidget` "/Game/Blueprints/HUD/TextToDisplay_BP.TextToDisplay_BP_C" null null self))
  (`UserWidget.AddToViewport` _returnvalue 0))

(fn `UserConstructionScript`)